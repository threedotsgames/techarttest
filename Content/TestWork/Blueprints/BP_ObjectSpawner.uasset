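; Spawner that scatters static mesh actors inside a box volume on BeginPlay or when SpawnObjects is called with new settings.
; A seeded random stream drives position, rotation (optionally yaw-only) and uniform scale.
; With AlignToGround, a downward Visibility trace places each mesh on the hit point, skipping misses.
; Spawned meshes ignore Visibility to prevent stacking and are tracked so SpawnObjects can destroy them before respawning.
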(event `SpawnObjects`
  (params (Seed :type Integer) (ObjCount :type Integer) (MaxScale :type "Float (double-precision)") (MinScale :type "Float (double-precision)"))
  (bind _randomstream (`self.RandomStream`))
  (bind _returnvalue (`KismetMathLibrary.RandomRotatorFromStream` _randomstream))
  (bind (_origin _boxextent) (`KismetSystemLibrary.GetComponentBounds` (`self.Box`)))
  (bind _returnvalue_2 (`KismetMathLibrary.RandomPointInBoundingBoxFromStream` _randomstream _origin _boxextent))
  ; Respawn from utility widget
  (for _array_element (`self.SpawnedActors`)
    (`self.K2_DestroyActor` _array_element))
  (set `self.Seed` Seed)
  (set `self.ObjCount` ObjCount)
  (set `self.MaxScale` MaxScale)
  (set `self.MinScale` MinScale)
  ;[0.0911 0.3125 0.1596 0.5] Generate random stream from seed for consistent results
  (set `self.RandomStream` (`KismetMathLibrary.MakeRandomStream` (`self.Seed`)) :!label _label)
  (for _ (range (`self.ObjCount`))
    (if (`self.AlignToGround`)
      ;[0.2656 0.2394 0.1383 0.5] Trace a ray to find the ground
      (bind _outhit (`KismetSystemLibrary.LineTraceSingle` _returnvalue_2 (- _returnvalue_2 (`KismetMathLibrary.MakeVector` 0.0 0.0 (.z _boxextent))) "TraceTypeQuery1"))
      (bind (_bblockinghit _binitialoverlap _time _distance _location _impactpoint) (`GameplayStatics.BreakHitResult` _outhit))
      (if _bblockinghit
        ; Spawn actor, save to array and remove visibility collision to prevent other actors from spawning on top
        (bind _returnvalue_3 (`|SpawnActorFromClass` "/Script/Engine.StaticMeshActor" (`KismetMathLibrary.MakeTransform` (`KismetMathLibrary.SelectVector` _impactpoint _returnvalue_2 (`self.AlignToGround`)) (`KismetMathLibrary.SelectRotator` (`KismetMathLibrary.MakeRotator` 0.0 0.0 (.yaw _returnvalue)) _returnvalue (`self.RotateOnlyZ`)) (`KismetMathLibrary.Conv_DoubleToVector` (`KismetMathLibrary.RandomFloatInRangeFromStream` _randomstream (`self.MinScale`) (`self.MaxScale`)))) "Undefined" "MultiplyWithRoot" null null :!label _label_2))
        (`KismetArrayLibrary.Array_Add` (`self.SpawnedActors`) _returnvalue_3)
        (bind _staticmeshcomponent (`StaticMeshActor.StaticMeshComponent` _returnvalue_3))
        (`StaticMeshComponent.SetStaticMesh` _staticmeshcomponent (`self.Mesh`))
        (`PrimitiveComponent.SetCollisionResponseToChannel` _staticmeshcomponent "ECC_Visibility" "ECR_Ignore"))
      (else
        (goto _label_2)))))

(event `self.ReceiveBeginPlay`
  (goto _label))

(fn `UserConstructionScript`)